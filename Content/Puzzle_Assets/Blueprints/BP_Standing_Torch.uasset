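; Standing torch prop for a puzzle asset set, with a point light built to flicker like fire.
; BeginPlay toggles the light's visibility after a short random delay, and Tick re-randomizes the flicker timeline's play rate every frame.
; The timeline's update scales its track by a random factor to set light intensity, but no wire in the graph starts it.
; A random start-time node is left unconnected.
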(event `self.ReceiveBeginPlay`
  (`KismetSystemLibrary.Delay` (`KismetMathLibrary.RandomFloatInRange` 2.0 4.0))
  (`SceneComponent.ToggleVisibility` (`self.PointLight`) false)
  (`TimelineComponent.SetPlayRate` (`self.FlickerTimeline`) (`KismetMathLibrary.RandomFloatInRange` 0.2 1.6) :!label _label))

(event `self.ReceiveTick`
  (params (DeltaSeconds :type "Float (single-precision)"))
  (goto _label))

(fn `UserConstructionScript`)