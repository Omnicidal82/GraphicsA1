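; BP_Dungeon_Torch is a dungeon torch with a flickering point light and flame audio.
; BeginPlay waits a random delay, plays a woosh at world origin and toggles the light's visibility.
; Tick randomizes FlickerTimeline's play rate, and timeline updates drive jittered light intensity and delayed crackles with random start offsets.
; No node in the graph starts the timeline, and its random SetNewTime node is unconnected.
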(event `self.ReceiveTick`
  (params (DeltaSeconds :type "Float (single-precision)"))
  ; Handles the core light flickering by multiplying the Timeline output with a random multiplier to ensure non-uniform brightness. Additionally, it triggers a randomized Flame_crackle sound effect with a staggered delay to prevent audio looping patterns, creating a natural, organic ambient atmosphere for the torch.
  (`TimelineComponent.SetPlayRate` (`self.FlickerTimeline`) (`KismetMathLibrary.RandomFloatInRange` 0.2 1.6) :!label _label))

(event `self.ReceiveBeginPlay`
  ; Handles the core light flickering by multiplying the Timeline output with a random multiplier to ensure non-uniform brightness. Additionally, it triggers a randomized Flame_crackle sound effect with a staggered delay to prevent audio looping patterns, creating a natural, organic ambient atmosphere for the torch.
  (`KismetSystemLibrary.Delay` (`KismetMathLibrary.RandomFloatInRange` 2.0 4.0))
  (`GameplayStatics.PlaySoundAtLocation` "/Game/Puzzle_Assets/SFX/Flame_woosh.Flame_woosh" (0.0 0.0 0.0) (struct) 1.0 1.0 0.0 null null null null)
  (`SceneComponent.ToggleVisibility` (`self.PointLight`) false)
  (goto _label))

(fn `UserConstructionScript`)