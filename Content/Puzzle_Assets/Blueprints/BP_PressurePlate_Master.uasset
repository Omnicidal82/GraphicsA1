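; Master pressure plate for a weight puzzle, checking whether an overlapping block or player character matches its required Weight ID.
; A dynamic material, created after a randomised startup delay, glows gold for a match, blue for underweight or red for overweight, with a pitched MetaSound tone.
; Matches set the PlateID's flag on BP_PuzzleManager and trigger its completion check.
; Leaving resets glow, sound and flag, then rechecks completion.
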(event `self.ReceiveBeginPlay`
  (bind _sm_platebase (`self.SM_PlateBase`))
  ; Executes a delayed startup sequence (5–6 seconds) to play an ignition sound and toggle the plate's visibility. It simultaneously creates a Dynamic Material Instance for SM_Plate_Base, storing it as Plate Glow MID to allow for real-time color changes during gameplay.
  (`KismetSystemLibrary.Delay` (`KismetMathLibrary.RandomFloatInRange` 5.0 6.0))
  (`GameplayStatics.SpawnSoundAtLocation` "/Game/Puzzle_Assets/SFX/Magic_woosh.Magic_woosh" (0.0 0.0 0.0) (struct) 1.0 1.0 0.5 null null)
  (`SceneComponent.ToggleVisibility` _sm_platebase false)
  (bind _returnvalue (`PrimitiveComponent.CreateDynamicMaterialInstance` _sm_platebase 0 null "None"))
  (set `self.PlateGlow_MID` _returnvalue))

(event `self.Box.OnComponentBeginOverlap`
  (params (OverlappedComponent :type "PrimitiveComponent Object Reference") (OtherActor :type "Actor Object Reference") (OtherComp :type "PrimitiveComponent Object Reference") (OtherBodyIndex :type Integer) (bFromSweep :type Boolean) (SweepResult :type "HitResult Structure (by ref)"))
  (bind _ms_platelights (`self.MS_PlateLights`))
  (bind _requiredweightid (`self.RequiredWeightID`))
  (bind _plateglow_mid (`self.PlateGlow_MID`))
  (bind _ms_platelights_2 (`self.MS_PlateLights`))
  ; Initiates when a player or block overlaps the plate, comparing their Weight ID against the target requirement to determine the puzzle state. It provides immediate feedback by updating the Plate Glow MID color—Green for success, Blue for underweight, or Red for overweight—while playing a corresponding audio tone via SwitchPitch. Finally, it updates the specific Plate Active boolean and calls the Puzzle Manager to check for overall completion.
  (`/Engine/EditorBlueprintResources/StandardMacros.IsValid` OtherActor
    (:`Is Valid`
      (bind _asbp_block_master (cast `/Game/Puzzle_Assets/Blueprints/BP_Block_Master` OtherActor)
        (:`then`
          (set `self.BlockCastSucceeded` true))
        (:`CastFailed`
          (`/Engine/EditorBlueprintResources/StandardMacros.IsValid` OtherActor
            (:`Is Valid`
              (bind _asbp_third_person_character (cast `/Game/ThirdPerson/Blueprints/BP_ThirdPersonCharacter` OtherActor))
              (set `self.BlockCastSucceeded` false)))))
      (bind _returnvalue (select `int` (`KismetMathLibrary.Conv_BoolToInt` (`self.BlockCastSucceeded`)) :`0` (`/Game/ThirdPerson/Blueprints/BP_ThirdPersonCharacter.WeightID` _asbp_third_person_character) :`1` (`/Game/Puzzle_Assets/Blueprints/BP_Block_Master.WeightID` _asbp_block_master)))
      (if (== _returnvalue _requiredweightid)
        (`MaterialInstanceDynamic.SetVectorParameterValue` _plateglow_mid "GlowColour" (make `LinearColor` 100.0 70.0 0.0 1.0))
        (`AudioComponent.SetFloatParameter` _ms_platelights_2 "SwitchPitch" 440.0)
        (`AudioComponent.Play` _ms_platelights_2 0.0)
        (bind _outactors (`GameplayStatics.GetAllActorsOfClass` "/Game/Puzzle_Assets/Blueprints/BP_PuzzleManager.BP_PuzzleManager_C"))
        (switch `int` (`self.PlateID`)
          (:`1`
            (bind _output (`|GetArrayItem` _outactors))
            (set `/Game/Puzzle_Assets/Blueprints/BP_PuzzleManager.Plate1_Active` true _output))
          (:`2`
            (set `/Game/Puzzle_Assets/Blueprints/BP_PuzzleManager.Plate2_Active` true _output))
          (:`3`
            (set `/Game/Puzzle_Assets/Blueprints/BP_PuzzleManager.Plate3_Active` true _output)))
        (`/Game/Puzzle_Assets/Blueprints/BP_PuzzleManager.Check_Puzzle_Completion` _outactors)
        (elif (< _returnvalue _requiredweightid)
          (`MaterialInstanceDynamic.SetVectorParameterValue` _plateglow_mid "GlowColour" (make `LinearColor` 0.0 0.0 170.0 1.0))
          (`AudioComponent.SetFloatParameter` _ms_platelights "SwitchPitch" 659.2)
          (`AudioComponent.Play` (`self.MS_PlateLights`) 0.0 :!label _label)
          (elif (> _returnvalue _requiredweightid)
            (`MaterialInstanceDynamic.SetVectorParameterValue` _plateglow_mid "GlowColour" (make `LinearColor` 170.0 0.0 0.0 1.0))
            (`AudioComponent.SetFloatParameter` _ms_platelights "SwitchPitch" 220.0)
            (goto _label)))))))

(event `self.Box.OnComponentEndOverlap`
  (params (OverlappedComponent :type "PrimitiveComponent Object Reference") (OtherActor :type "Actor Object Reference") (OtherComp :type "PrimitiveComponent Object Reference") (OtherBodyIndex :type Integer))
  ; Handles the visual and logical reset when a valid actor leaves the plate. It sets the GlowColour back to its default state, stops associated audio, and updates the Puzzle Manager to mark this specific plate as inactive, prompting a re-check of the door or puzzle status.
  (`/Engine/EditorBlueprintResources/StandardMacros.IsValid` OtherActor
    (:`Is Valid`
      (cast `/Game/Puzzle_Assets/Blueprints/BP_Block_Master` OtherActor
        (:`then`
          _)
        (:`CastFailed`
          (`/Engine/EditorBlueprintResources/StandardMacros.IsValid` OtherActor
            (:`Is Valid`
              (cast `/Game/ThirdPerson/Blueprints/BP_ThirdPersonCharacter` OtherActor)))))
      (bind _outactors (`GameplayStatics.GetAllActorsOfClass` "/Game/Puzzle_Assets/Blueprints/BP_PuzzleManager.BP_PuzzleManager_C"))
      (`MaterialInstanceDynamic.SetVectorParameterValue` (`self.PlateGlow_MID`) "GlowColour" (make `LinearColor` 0.093059 0.904661 0.198069 1.0))
      (`AudioComponent.Stop` (`self.MS_PlateLights`))
      (switch `int` (`self.PlateID`)
        (:`1`
          (bind _output (`|GetArrayItem` _outactors))
          (set `/Game/Puzzle_Assets/Blueprints/BP_PuzzleManager.Plate1_Active` false _output))
        (:`2`
          (set `/Game/Puzzle_Assets/Blueprints/BP_PuzzleManager.Plate2_Active` false _output))
        (:`3`
          (set `/Game/Puzzle_Assets/Blueprints/BP_PuzzleManager.Plate3_Active` false _output)))
      (`/Game/Puzzle_Assets/Blueprints/BP_PuzzleManager.Check_Puzzle_Completion` _outactors))))

(fn `UserConstructionScript`)